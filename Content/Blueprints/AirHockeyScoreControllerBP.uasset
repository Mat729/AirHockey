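; Air hockey goal controller that recycles the disk when it enters either goal; no score is tracked in this graph.
; It binds both goals' overlap events on BeginPlay, checking only Goal1's validity, then destroys an overlapping disk and calls SpawnDisk.
; A separate RespawnDisk event sphere-checks the spawn point for paddles, retrying on a delay until clear before spawning.
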(event Custom|Goal
  (params (OverlappedActor :type Actor%20Object%20Reference) (OtherActor :type Actor%20Object%20Reference))
  (bind _asair_hockey_disk (Utilities|Casting|CastToAirHockeyDisk OtherActor))
  (Actor|DestroyActor _asair_hockey_disk)
  (Class|AirHockeyDiskSpawner|SpawnDisk))

(event Custom|RespawnDisk
  (if (Utilities|IsValid (Variables|Default|GetDiskSpawnPoint))
    (Development|PrintString "Trying spawn a new Disk..." true true "(R=1.000000,G=1.000000,B=1.000000,A=1.000000)" 3e+01 :!label _label)
    (bind _returnvalue (Collision|SphereOverlapActors (Transformation|GetActorLocation (Variables|Default|GetDiskSpawnPoint)) (Variables|Default|GetSpawnRadius) (Variables|Default|GetFilter) "/Script/AirHockeyPhysics.AirHockeyPaddle"))
    (if _returnvalue
      (Development|PrintString "Obstacle Found. Retrying in a while..." true true "(R=1.000000,G=0.000000,B=0.000000,A=1.000000)" 3e+01)
      (Utilities|FlowControl|Delay 2.0)
      (goto _label)
      (else
        (Class|AirHockeyDiskSpawner|SpawnDisk)
        (Development|PrintString "Disk spawned" true true "(R=0.000000,G=1.000000,B=0.000000,A=1.000000)" 3e+01)))))

(event EventBeginPlay
  ;[1 1 1] BeginPlay
  (Utilities|FlowControl|Sequence
    (:then_0
      (if (Utilities|IsValid (Variables|Default|GetGoal1))
        (Collision|BindEventtoOnActorBeginOverlap (Variables|Default|GetGoal1) (delegate Custom|Goal))))
    (:then_1
      (if (Utilities|IsValid (Variables|Default|GetGoal1))
        (Collision|BindEventtoOnActorBeginOverlap (Variables|Default|GetGoal2) (delegate Custom|Goal))))))

(event EventEndPlay
  (params (EndPlayReason :type EEndPlayReason%20Enum :default "Destroyed"))
  ;[1 1 1] EndPlay
  (Utilities|FlowControl|Sequence
    (:then_0
      (if (Utilities|IsValid (Variables|Default|GetGoal1))
        (Collision|UnbindEventfromOnActorBeginOverlap (Variables|Default|GetGoal1) (delegate Custom|Goal))))
    (:then_1
      (if (Utilities|IsValid (Variables|Default|GetGoal1))
        (Collision|UnbindEventfromOnActorBeginOverlap (Variables|Default|GetGoal2) (delegate Custom|Goal))))))

(fn ConstructionScript)